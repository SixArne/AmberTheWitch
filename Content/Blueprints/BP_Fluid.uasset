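; BP_Fluid animates a fluid segment as a spline mesh that travels along a referenced spline and shrinks as it goes.
; On BeginPlay it adds a Z-forward spline mesh component to the Spline object, then plays FluidTimeline at a rate set by Duration.
; Each timeline update offsets StartTime and EndTime by Alpha to resample positions and tangents, and tapers both end scales as Alpha rises.
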(event Custom|AddSplineMesh
  (bind _starttime (Variables|Default|GetStartTime))
  (bind _alpha (Variables|Default|GetAlpha))
  (bind _alpha_2 (Variables|Default|GetAlpha))
  (bind _alpha_3 (Variables|Default|GetAlpha))
  (bind _endtime (Variables|Default|GetEndTime))
  (bind _endtime_2 (Variables|Default|GetEndTime))
  (bind _spline (Variables|Default|GetSpline))
  (bind _returnvalue (+ _starttime _alpha))
  (bind _returnvalue_2 (+ _endtime_2 _alpha))
  (bind _returnvalue_3 (+ _alpha_3 _endtime))
  (bind _returnvalue_4 (- 1.0 _alpha_2))
  (bind _spline_2 (Variables|/Game/Blueprints/BP_FluidSpline.BP_FluidSpline_C|GetSpline _spline))
  (bind _returnvalue_5 (- 1.0 _returnvalue_3))
  (bind _returnvalue_6 (AddComponent|AddSplineMeshComponent (Variables|Default|GetSpline) true))
  (bind _output_get (Variables|Default|SetSplineMesh _returnvalue_6))
  (SplineMesh|SetForwardAxis _output_get "Z" true)
  (SplineMesh|SetStartandEnd _output_get (Spline|GetLocationatTime _spline_2 _returnvalue "World" false) (Class|SplineComponent|GetTangentatTime _spline_2 _returnvalue "World" false) (Spline|GetLocationatTime _spline_2 _returnvalue_2 "World" false) (Class|SplineComponent|GetTangentatTime _spline_2 _returnvalue_2 "World" false) true :!class /Script/Engine.SplineMeshComponent)
  (SplineMesh|SetStartScale _output_get (Math|Vector2D|MakeVector2D _returnvalue_4 _returnvalue_4) true :!class /Script/Engine.SplineMeshComponent)
  (SplineMesh|SetEndScale _output_get (Math|Vector2D|MakeVector2D _returnvalue_5 _returnvalue_5) true :!class /Script/Engine.SplineMeshComponent))

(event Custom|MoveSplineMesh
  (Components|Timeline|SetPlayRate (Variables|Default|GetFluidTimeline) (/ 1.0 (Variables|Default|GetDuration)))
  (bind _alpha (Timeline|FluidTimeline Play)
    (:Update
      (Variables|Default|SetAlpha _alpha)
      (CallFunction|UpdateMesh))))

(event Custom|UpdateMesh
  (bind _starttime (Variables|Default|GetStartTime))
  (bind _alpha (Variables|Default|GetAlpha))
  (bind _alpha_2 (Variables|Default|GetAlpha))
  (bind _alpha_3 (Variables|Default|GetAlpha))
  (bind _endtime (Variables|Default|GetEndTime))
  (bind _endtime_2 (Variables|Default|GetEndTime))
  (bind _spline (Variables|Default|GetSpline))
  (bind _returnvalue (+ _starttime _alpha))
  (bind _returnvalue_2 (+ _endtime_2 _alpha))
  (bind _returnvalue_3 (+ _alpha_3 _endtime))
  (bind _returnvalue_4 (- 1.0 _alpha_2))
  (bind _spline_2 (Variables|/Game/Blueprints/BP_FluidSpline.BP_FluidSpline_C|GetSpline _spline))
  (bind _returnvalue_5 (- 1.0 _returnvalue_3))
  (Utilities|IsValid (Variables|Default|GetSpline)
    (:Is%20Valid
      (SplineMesh|SetStartandEnd (stale Custom|AddSplineMesh _output_get) (Spline|GetLocationatTime _spline_2 _returnvalue "World" false) (Class|SplineComponent|GetTangentatTime _spline_2 _returnvalue "World" false) (Spline|GetLocationatTime _spline_2 _returnvalue_2 "World" false) (Class|SplineComponent|GetTangentatTime _spline_2 _returnvalue_2 "World" false) true :!class /Script/Engine.SplineMeshComponent)
      (SplineMesh|SetStartScale (stale Custom|AddSplineMesh _output_get) (Math|Vector2D|MakeVector2D _returnvalue_4 _returnvalue_4) true :!class /Script/Engine.SplineMeshComponent)
      (SplineMesh|SetEndScale (stale Custom|AddSplineMesh _output_get) (Math|Vector2D|MakeVector2D _returnvalue_5 _returnvalue_5) true :!class /Script/Engine.SplineMeshComponent))))

(event EventBeginPlay
  (CallFunction|AddSplineMesh)
  (CallFunction|MoveSplineMesh))

(fn ConstructionScript)