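; BP_Flask is a flask actor that spawns and manages its own detachable BP_Cork, with configurable meshes for both.
; On BeginPlay it spawns the cork at CorkSocket, attaches it, links it back to itself and applies its mesh.
; While IsAttached is set, Tick sweeps the cork to the socket transform.
; Grab and release events toggle cork physics off and on, and destroying the flask destroys the cork.
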(event Custom|OnReleasedCork
  ;[1 1 1] gravity = on: on dropping cork
  (Physics|SetSimulatePhysics (Variables|/Game/Blueprints/BP_Cork.BP_Cork_C|GetCork (Variables|Default|GetCork)) true))

(event Custom|OnGrabCork
  ;[1 1 1] gravity = off :on Grabbing cork
  (Physics|SetSimulatePhysics (Variables|/Game/Blueprints/BP_Cork.BP_Cork_C|GetCork (Variables|Default|GetCork)) false))

(event Custom|OnDestroyed_Event
  (params (DestroyedActor :type Actor%20Object%20Reference))
  (Utilities|FlowControl|Sequence
    (:then_0
      (bind _cork (Variables|Default|GetCork)
        (:then
          (Actor|DestroyActor _cork))
        (:else)))
    (:then_1
      (Actor|DestroyActor))))

(event EventBeginPlay
  (Game|AssignOnDestroyed (delegate Custom|OnDestroyed_Event))
  ;[1 1 1] Spawning cork on begin
  (bind _returnvalue (Game|SpawnActorfromClass "/Game/Blueprints/BP_Cork.BP_Cork_C" (Transformation|GetWorldTransform (Variables|Default|GetCorkSocket)) "AlwaysSpawn" 0 0))
  (bind _output_get (Variables|Default|SetCork _returnvalue))
  (Utilities|AttachCorktoFlask _output_get)
  (Variables|/Game/Blueprints/BP_Cork.BP_Cork_C|SetFlask (Variables|Default|GetCork) self)
  (Components|StaticMesh|SetStaticMesh (Variables|/Game/Blueprints/BP_Cork.BP_Cork_C|GetCork (Variables|Default|GetCork)) (Variables|_Settings|GetCorkMesh)))

(event Collision|EventActorBeginOverlap
  (params (OtherActor :type Actor%20Object%20Reference)))

(event EventTick
  (params (DeltaSeconds :type Float%20%28single-precision%29))
  ;[1 1 1] Set position
  (if (Variables|Default|GetIsAttached)
    (Transformation|SetActorTransform (Variables|Default|GetCork) (Transformation|GetWorldTransform (Variables|Default|GetCorkSocket)) true)))

(fn ConstructionScript
  (Utilities|FlowControl|Sequence
    (:then_0
      (Components|StaticMesh|SetStaticMesh (Variables|/Game/Blueprints/BP_Cork.BP_Cork_C|GetCork (Variables|Default|GetCork)) (Variables|_Settings|GetCorkMesh)))
    (:then_1
      (Components|StaticMesh|SetStaticMesh (Variables|Default|Getflask) (Variables|_Settings|GetFlaskMesh)))))